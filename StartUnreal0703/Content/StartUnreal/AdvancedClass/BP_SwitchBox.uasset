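; BP_SwitchBox is a trigger switch that starts and stops every EventComponent-equipped actor in the level.
; A begin overlap on its Cube scans all actors and calls DoPlay on the EventComponent found on each.
; The actor-level end overlap repeats the scan and calls StopPlay.
; Neither event filters the overlapping actor, and both search the whole level each time rather than caching targets.
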(event OnComponentBeginOverlap(Cube)
  (params (OverlappedComponent :type Primitive%20Component%20Object%20Reference) (OtherActor :type Actor%20Object%20Reference) (OtherComp :type Primitive%20Component%20Object%20Reference) (OtherBodyIndex :type Integer) (bFromSweep :type Boolean) (SweepResult :type Hit%20Result%20Structure%20%28by%20ref%29))
  (bind _outactors (Actor|GetAllActorsOfClass "/Script/Engine.Actor"))
  (for _array_element _outactors
    (Utilities|IsValid (Actor|GetComponentbyClass _array_element "/Game/StartUnreal/AdvancedClass/EventComponent.EventComponent_C")
      (:Is%20Valid
        (Default|DoPlay (Actor|GetComponentbyClass _array_element "/Game/StartUnreal/AdvancedClass/EventComponent.EventComponent_C"))))))

(event Collision|EventActorEndOverlap
  (params (OtherActor :type Actor%20Object%20Reference))
  (bind _outactors (Actor|GetAllActorsOfClass "/Script/Engine.Actor"))
  (for _array_element _outactors
    (Utilities|IsValid (Actor|GetComponentbyClass _array_element "/Game/StartUnreal/AdvancedClass/EventComponent.EventComponent_C")
      (:Is%20Valid
        (Default|StopPlay (Actor|GetComponentbyClass _array_element "/Game/StartUnreal/AdvancedClass/EventComponent.EventComponent_C"))))))

(fn ConstructionScript)