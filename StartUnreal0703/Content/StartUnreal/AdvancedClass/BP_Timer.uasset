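; BP_Timer is an actor that shows elapsed time as a zero-padded MM:SS readout on a TextRender.
; EventComponent's play and stop dispatchers toggle IsAvailable, which gates Tick accumulation of delta seconds without resetting the total.
; The FloatToString00 helper floors and pads the minutes and seconds values.
; Two disconnected graphs keep earlier approaches, one using per-digit carry counters and one using inline branching.
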(event EventDispatcherDoPlay(EventComponent)
  (Variables|Default|SetIsAvailable true))

(event EventDispatcherStopPlay(EventComponent)
  (Variables|Default|SetIsAvailable false))

(event EventTick
  (params (DeltaSeconds :type Float%20%28single-precision%29))
  ;[1 1 1] 함수를 사용한다면?
  (if (Variables|Default|GetIsAvailable)
    (bind _output_get (Variables|Default|SetNewVar_0 (+ DeltaSeconds (Variables|Default|GetNewVar_0))))
    (Rendering|Components|TextRender|SetText (Variables|Default|GetTextRender) (Utilities|Text|ToText(String) (Utilities|String|Append (Func|FloattoString00 (/ _output_get 6e+01)) ":" (Func|FloattoString00 (Math|Float|%(Float) _output_get 6e+01)))))))

(fn ConstructionScript)

(fn FloattoString00
  (params (InputNumber :type Float%20%28double-precision%29))
  (bind _returnvalue (Math|Float|Floor InputNumber))
  (bind _returnvalue_2 (Utilities|String|ToString(Integer) _returnvalue))
  (if (< _returnvalue 10)
    (return (Utilities|String|Append "0" _returnvalue_2))
    (else
      (return _returnvalue_2))))