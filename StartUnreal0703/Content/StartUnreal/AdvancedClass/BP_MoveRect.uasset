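; BP_MoveRect moves its Cube around a square loop in the local XZ plane while IsAvailable is true.
; Tick runs a MoveType state machine that steps the cube a fixed amount per frame, not scaled by delta time, switching direction at each bound.
; EventComponent play/stop dispatchers and an overlap-driven function toggle IsAvailable.
; An unconnected Timeline that would set the cube's X location never runs.
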(event EventDispatcherDoPlay(EventComponent)
  (Variables|Default|SetIsAvailable true))

(event EventDispatcherStopPlay(EventComponent)
  (Variables|Default|SetIsAvailable false))

(event EventTick
  (params (DeltaSeconds :type Float%20%28single-precision%29))
  (bind _cube (Variables|Default|GetCube))
  (bind _cube_2 (Variables|Default|GetCube))
  (bind _cube_3 (Variables|Default|GetCube))
  (if (Variables|Default|GetIsAvailable)
    (switch Utilities|FlowControl|Switch|SwitchonEN_MoveType (Variables|Default|GetMove%20Type)
      (:NewEnumerator0
        ;[1 1 1] Right
        (bind _returnvalue (CallFunction|MoveRight))
        (if _returnvalue
          (Variables|Default|SetMove%20Type "NewEnumerator1")))
      (:NewEnumerator1
        ;[1 1 1] Up
        (Transformation|AddRelativeLocation _cube_2 "0.000000,0.000000,1.000000" false false)
        (if (> (.z (Variables|/Script/Engine.SceneComponent|GetRelativeLocation _cube_2)) 1e+02)
          (Variables|Default|SetMove%20Type "NewEnumerator2")))
      (:NewEnumerator2
        ;[1 1 1] Left
        (Transformation|AddRelativeLocation _cube_3 "-1.000000,0.000000,0.000000" false false)
        (if (< (.x (Variables|/Script/Engine.SceneComponent|GetRelativeLocation _cube_3)) 0.0)
          (Variables|Default|SetMove%20Type "NewEnumerator3")))
      (:NewEnumerator3
        ;[1 1 1] Down
        (Transformation|AddRelativeLocation _cube "0.000000,0.000000,-1.000000" false false)
        (if (< (.z (Variables|/Script/Engine.SceneComponent|GetRelativeLocation _cube)) 0.0)
          (Variables|Default|SetMove%20Type "NewEnumerator0"))))))

(fn ConstructionScript)

(fn BPMoveRectAutoGenFunc
  (params (IsBeginOverlap :type Boolean))
  (Variables|Default|SetIsAvailable IsBeginOverlap))

(fn MoveRight
  (bind _cube (Variables|Default|GetCube))
  (Transformation|AddRelativeLocation _cube "1.000000,0.000000,0.000000" false false)
  (return (> (.x (Variables|/Script/Engine.SceneComponent|GetRelativeLocation _cube)) 1e+02)))