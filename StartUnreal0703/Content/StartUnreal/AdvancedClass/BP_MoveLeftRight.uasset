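; BP_MoveLeftRight is an actor Blueprint that slides its Sphere component back and forth along its relative X axis while playing.
; Tick moves the offset one unit per frame, independent of delta time, and flips IsMoveLeft when it passes either end of the range.
; DoPlay and StopPlay override parent functions, calling them before toggling IsPlay to gate the motion.
; A switch on MoveType is left unconnected.
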(event EventTick
  (params (DeltaSeconds :type Float%20%28single-precision%29))
  (if (Variables|Default|GetIsPlay)
    (if (Variables|Default|GetIsMoveLeft)
      ;[1 1 1] Move Right
      (bind _output_get (Variables|Default|SetThat (+ (Variables|Default|GetThat) 1.0)))
      (Transformation|SetRelativeLocation (Variables|Default|GetSphere) (Math|Vector|MakeVector _output_get 0.0 0.0) false false)
      (if (> (Variables|Default|GetThat) 1e+02)
        (Variables|Default|SetIsMoveLeft false))
      (else
        ;[1 1 1] Move Right
        (bind _output_get_2 (Variables|Default|SetThat (+ (Variables|Default|GetThat) -1.0)))
        (Transformation|SetRelativeLocation (Variables|Default|GetSphere) (Math|Vector|MakeVector _output_get_2 0.0 0.0) false false)
        (if (< (Variables|Default|GetThat) 0.0)
          (Variables|Default|SetIsMoveLeft true))))))

(fn ConstructionScript)

(fn DoPlay
  (|CallParentFunction)
  (Variables|Default|SetIsPlay true))

(fn StopPlay
  (|CallParentFunction)
  (Variables|Default|SetIsPlay false))